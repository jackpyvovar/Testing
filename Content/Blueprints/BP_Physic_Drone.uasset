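; Player-controlled physics drone pawn that flies, shoots projectiles and tracks health and ammo.
; Mass-scaled thruster force drives lift, with the mesh's center of mass shifted under the thruster on BeginPlay.
; Axis inputs apply torque for yaw and clamped, rotation-corrected tilt, while mouse input pitches the spring arm.
; Shots follow camera rotation; hit and pickup events adjust stats, print them, and destroy the drone at zero health.
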(event `InputAxis|Mouse Up`
  (params (AxisValue :type "Float (single-precision)"))
  ;[1 1 1] Camera
  (`SceneComponent.K2_AddRelativeRotation` (`self.SpringArm`) (`KismetMathLibrary.MakeRotator` 0.0 AxisValue) false false))

(event `InputAxis|Move Up`
  (params (AxisValue :type "Float (single-precision)"))
  ;[1 1 1] Move Up/Down
  (set `PhysicsThrusterComponent.ThrustStrength` (* (* (* AxisValue 100.0) 20.0) (`PrimitiveComponent.GetMass` (`self.StaticMesh`))) (`self.PhysicsThruster`)))

(event `self.ReceiveBeginPlay`
  (bind (_returnvalue_x _returnvalue_y) (`KismetMathLibrary.BreakVector` (`KismetMathLibrary.GreaterGreater_VectorRotator` (- (`SceneComponent.K2_GetComponentLocation` (`self.PhysicsThruster`)) (`PrimitiveComponent.GetCenterOfMass` (`self.StaticMesh`) "None")) (`KismetMathLibrary.NegateRotator` (`SceneComponent.K2_GetComponentRotation` (`self.StaticMesh`))))))
  (`|ExecutionSequence`
    (:`then_0`
      ;[1 1 1] Center mass
      (`PrimitiveComponent.SetCenterOfMass` (`self.StaticMesh`) (`KismetMathLibrary.MakeVector` _returnvalue_x _returnvalue_y) "None"))
    (:`then_1`
      ;[1 1 1] HP Bar
      (bind _returnvalue (`|CreateWidget` "/Game/Blueprints/BP_HealthBar.BP_HealthBar_C"))
      (`UserWidget.AddToViewport` _returnvalue 0))))

(event `InputAxis|Rotate Right`
  (params (AxisValue :type "Float (single-precision)"))
  ;[1 1 1] Rotation
  (`PrimitiveComponent.AddTorqueInDegrees` (`self.StaticMesh`) (* AxisValue (`self.GetActorUpVector`) 1000.0) "None" true))

(event `InputAxis|Tilt Forward`
  (params (AxisValue :type "Float (single-precision)"))
  (bind (_returnvalue_roll _returnvalue_pitch) (`KismetMathLibrary.BreakRotator` (`SceneComponent.K2_GetComponentRotation` (`self.StaticMesh`))))
  ;[1 1 1] Tilt Forward
  (`PrimitiveComponent.AddTorqueInDegrees` (`self.StaticMesh`) (* (`self.GetActorRightVector`) (`KismetMathLibrary.FClamp` (+ (* AxisValue 40.0) _returnvalue_pitch) -40.0 40.0) 5.0) "None" true))

(event `InputAxis|Tilt Right`
  (params (AxisValue :type "Float (single-precision)"))
  (bind _returnvalue_roll (`KismetMathLibrary.BreakRotator` (`SceneComponent.K2_GetComponentRotation` (`self.StaticMesh`))))
  ;[1 1 1] Tilt Sideways
  (`PrimitiveComponent.AddTorqueInDegrees` (`self.StaticMesh`) (* (`self.GetActorForwardVector`) (`KismetMathLibrary.FClamp` (+ (* AxisValue -30.0) _returnvalue_roll) -20.0 20.0) 5.0) "None" true))

(event `Key|LeftMouseButton`
  (params (Key :type "Key Structure"))
  (bind _returnvalue (`PlayerCameraManager.GetCameraRotation` (`GameplayStatics.GetPlayerCameraManager` 0)))
  ;[1 1 1] Shoot
  (:`Pressed`
    (if (> (`self.Current Ammo`) 0)
      (`|SpawnActorFromClass` "/Game/Blueprints/BP_FirstPersonProjectileYou.BP_FirstPersonProjectileYou_C" (`KismetMathLibrary.MakeTransform` (+ (`SceneComponent.GetSocketLocation` (`self.Arrow`) "Ammo") (`KismetMathLibrary.GreaterGreater_VectorRotator` (`self.Projectile Offset`) _returnvalue)) _returnvalue) "Undefined" "OverrideRootScale" null null)
      (bind _result (`/Engine/EditorBlueprintResources/StandardMacros.DecrementInt` (`self.Current Ammo`))
        (:`  `
          (bind _output_get (set `self.Current Ammo` _result))
          (`KismetSystemLibrary.PrintString` (`KismetStringLibrary.Conv_IntToString` _output_get) true true (struct :`R` 1.0 :`G` 0.764706 :`A` 1.0))))
      (else
        (`KismetSystemLibrary.PrintString` "No Ammo" true true (struct :`R` 1.0 :`G` 0.764706 :`A` 1.0))))))

(event `Event You Hit`
  (params (Damage :type "Float (double-precision)"))
  ;[1 1 1] HP
  (bind _output_get (set `self.Health` (- (`self.Health`) Damage)))
  (if (<= _output_get 0.0)
    (`KismetSystemLibrary.PrintString` "You  Killed" true true (struct :`R` 1.0 :`A` 1.0))
    (`self.K2_DestroyActor`)
    (else
      (`KismetSystemLibrary.PrintString` (`KismetStringLibrary.Conv_DoubleToString` _output_get) true true (struct :`R` 1.0 :`A` 1.0)))))

(event `Increase health`
  ;[1 1 1] Pack
  ;;[1 0 0] Health
  (set `self.Health` (+ (`self.Health`) 20.0))
  (if (> (`self.Health`) (`self.Max Health`))
    (bind _output_get (set `self.Health` 100.0))
    (`KismetSystemLibrary.PrintString` (`KismetStringLibrary.Conv_DoubleToString` _output_get) true true (struct :`R` 1.0 :`A` 1.0))
    (else
      (`KismetSystemLibrary.PrintString` (`KismetStringLibrary.Conv_DoubleToString` (`self.Health`)) true true (struct :`R` 1.0 :`A` 1.0)))))

(event `Increase Ammo`
  ;[1 1 1] Pack
  ;;[1 0.844 0] Ammo
  (set `self.Current Ammo` (+ (`self.Current Ammo`) 10))
  (if (> (`self.Current Ammo`) (`self.Max Ammo`))
    (bind _output_get (set `self.Current Ammo` 100))
    (`KismetSystemLibrary.PrintString` (`KismetStringLibrary.Conv_IntToString` _output_get) true true (struct :`R` 1.0 :`G` 0.764706 :`A` 1.0))
    (else
      (`KismetSystemLibrary.PrintString` (`KismetStringLibrary.Conv_IntToString` (`self.Current Ammo`)) true true (struct :`R` 1.0 :`G` 0.764706 :`A` 1.0)))))

(fn `UserConstructionScript`)