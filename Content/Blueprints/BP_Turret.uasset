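; BP_Turret is an enemy turret that shoots at pawns it sees and can be destroyed.
; PawnSensing turns the actor toward any seen pawn except BP_Physic_Drone, then after a short Delay spawns an enemy projectile from its Arrow component.
; EnemyHit subtracts damage from Health, printing what remains or destroying the turret at zero or below.
; Casts to BP_ThirdPersonCharacter and BP_Drone remain in the graph but never run.
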(event `self.PawnSensing.OnSeePawn`
  (params (Pawn :type "Pawn Object Reference"))
  (cast `/Game/Blueprints/BP_Physic_Drone` Pawn
    (:`CastFailed`
      (`self.K2_SetActorRotation` (`KismetMathLibrary.FindLookAtRotation` (`self.K2_GetActorLocation`) (`self.K2_GetActorLocation` Pawn)))
      (`KismetSystemLibrary.Delay` 0.5)
      (`|SpawnActorFromClass` "/Game/Blueprints/BP_FirstPersonProjectileEnemy.BP_FirstPersonProjectileEnemy_C" (`SceneComponent.K2_GetComponentToWorld` (`self.Arrow`)) "Undefined" "MultiplyWithRoot" null null))))

(event `/Game/Blueprints/BP_EnemyDamageInterface.Enemy Hit`
  (params (Damage :type "Float (double-precision)"))
  (bind _output_get (set `self.Health` (- (`self.Health`) Damage)))
  (if (<= _output_get 0.0)
    (`KismetSystemLibrary.PrintString` "Enemy Killed")
    (`self.K2_DestroyActor`)
    (else
      (`KismetSystemLibrary.PrintString` (`KismetStringLibrary.Conv_DoubleToString` _output_get)))))

(fn `UserConstructionScript`)